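; Spurgu character Blueprint: a dagger-wielding attacker that damages the hero.
; Each attack start from the anim Blueprint clears the hit flag and removes the Damager from the hero's blocked damagers.
; The toggleable Damager collider applies damage once per attack, ignoring components on one custom collision channel.
; Grab and holster functions snap the knife between a virtual-bone hand socket and its holster socket.
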(event `self.ReceiveBeginPlay`
  ;[1 1 1] Init
  (`/Engine/EditorBlueprintResources/StandardMacros.IsValid` (`self.Animator`)
    (:`Is Valid`
      _)
    (:`Is Not Valid`
      (bind _output_get (set `self.Animator` (cast `/Game/Characters/Spurgu/Blueprints/SpurguAnimBP` (`SkeletalMeshComponent.GetAnimInstance` (`self.Mesh`)) :!pure true)))))
  (add `/Game/Characters/Spurgu/Blueprints/SpurguAnimBP.OnAnyAttackBegin` _output_get (delegate `OnAnyAttackBegin`)))

(event `OnAnyAttackBegin`
  ;[1 1 1] Init
  (set `self.hitHero` false)
  (bind _returnvalue (`self.FindHero`))
  (`HeroCharacter.RemoveBlockedDamager` _returnvalue (`self.Damager`)))

(event `self.Damager.OnComponentBeginOverlap`
  (params (OverlappedComponent :type "PrimitiveComponent Object Reference") (OtherActor :type "Actor Object Reference") (OtherComp :type "PrimitiveComponent Object Reference") (OtherBodyIndex :type Integer) (bFromSweep :type Boolean) (SweepResult :type "HitResult Structure (by ref)"))
  ;[1 1 1] Damage
  (bind _ashero_bp (cast `/Game/Characters/Sankari/Blueprints/HeroBP` OtherActor))
  (if (and (`|EnumInequality` (`PrimitiveComponent.GetCollisionObjectType` OtherComp) "ECC_GameTraceChannel2") (not (`self.hitHero`)))
    (set `self.hitHero` true)
    (set `self.activeDamager` (`self.Damager`))
    (`GameplayStatics.ApplyDamage` _ashero_bp (`KismetMathLibrary.Conv_IntToDouble` (`self.GetDamage`)) (`self.GetController`) self "/Script/Engine.DamageType")))

(event `self.EnableAttackColliders`
  (params (value :type Boolean) (colId :type Integer))
  (bind _damager (`self.Damager`))
  ;[1 1 1] Damage
  (if value
    (`PrimitiveComponent.SetCollisionEnabled` _damager "QueryOnly")
    (else
      (`PrimitiveComponent.SetCollisionEnabled` _damager "NoCollision"))))

(fn `GrabDagger`
  (bind _knife (`self.Knife`))
  (if (not (== (`SceneComponent.GetAttachSocketName` _knife) "VB hand_R_DEF_hand_R_DEF"))
    (`SceneComponent.K2_AttachToComponent` _knife (`self.Mesh`) "VB hand_R_DEF_hand_R_DEF" "SnapToTarget" "SnapToTarget" "KeepRelative" true)))

(fn `HolsterDagger`
  (bind _knife (`self.Knife`))
  (if (not (== (`SceneComponent.GetAttachSocketName` _knife) "knife_holster_socket"))
    (`SceneComponent.K2_AttachToComponent` _knife (`self.Mesh`) "knife_holster_socket" "SnapToTarget" "SnapToTarget" "KeepRelative" true)))

(fn `UserConstructionScript`)