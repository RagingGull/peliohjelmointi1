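; Hero character Blueprint handling melee axe attacks, cigar smoke stuns and blocking.
; The toggleable Damager volume applies current-attack damage once per actor, using a blacklist cleared whenever the animation Blueprint signals an attack start.
; Cigar smoke enables a timed volume that stuns basic enemies, both scaled by the supplied time.
; The Blocker volume interrupts enemy attacks while blocking, records the enemy and damager, and opens a timed counter window with debug prints.
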(event `self.ReceiveBeginPlay`
  (bind _returnvalue (`SkeletalMeshComponent.GetAnimInstance` (`self.Mesh`)))
  ;[1 1 1] Clear axe blacklist
  (`/Engine/EditorBlueprintResources/StandardMacros.IsValid` _returnvalue
    (:`Is Valid`
      (add `/Game/Characters/Sankari/Blueprints/HeroAnimationBP.OnAnyAttackBegin` (cast `/Game/Characters/Sankari/Blueprints/HeroAnimationBP` _returnvalue :!pure true) (delegate `ClearDamagerBlacklist`)))))

(event `ClearDamagerBlacklist`
  ;[1 1 1] Clear axe blacklist
  (`KismetArrayLibrary.Array_Clear` (`self.damagerBlacklist`)))

(event `self.Damager.OnComponentBeginOverlap`
  (params (OverlappedComponent :type "PrimitiveComponent Object Reference") (OtherActor :type "Actor Object Reference") (OtherComp :type "PrimitiveComponent Object Reference") (OtherBodyIndex :type Integer) (bFromSweep :type Boolean) (SweepResult :type "HitResult Structure (by ref)"))
  (bind (_returnvalue_damagetype _returnvalue_damage) (break `HeroAttackType` (`self.GetCurrentAttackType`)))
  ;[1 1 1] Axe damage
  (if (and (!= OtherActor self) (== (`GameplayStatics.GetObjectClass` OtherComp) "/Script/Engine.SkeletalMeshComponent") (not (`KismetArrayLibrary.Array_Contains` (`self.damagerBlacklist`) OtherActor)))
    (`GameplayStatics.ApplyDamage` OtherActor (`KismetMathLibrary.Conv_IntToDouble` _returnvalue_damage) (`self.GetController`) self _returnvalue_damagetype)
    (`KismetArrayLibrary.Array_Add` (`self.damagerBlacklist`) OtherActor)))

(event `self.OnCigarSmokeStart`
  (params (time :type "Float (single-precision)"))
  (bind _smokeduration (`self.smokeDuration`))
  ;[1 1 1] Smoke Damage
  (bind _output_get (set `self.smokeDurationMultiplier` (`KismetMathLibrary.FClamp` (/ time _smokeduration))))
  (`KismetSystemLibrary.K2_SetTimerDelegate` (delegate `SmokeEnd`) (* _smokeduration _output_get))
  (`PrimitiveComponent.SetCollisionEnabled` (`self.SmokeVolume`) "QueryOnly"))

(event `SmokeEnd`
  ;[1 1 1] Smoke Damage
  (`PrimitiveComponent.SetCollisionEnabled` (`self.SmokeVolume`) "NoCollision"))

(event `self.SmokeVolume.OnComponentBeginOverlap`
  (params (OverlappedComponent :type "PrimitiveComponent Object Reference") (OtherActor :type "Actor Object Reference") (OtherComp :type "PrimitiveComponent Object Reference") (OtherBodyIndex :type Integer) (bFromSweep :type Boolean) (SweepResult :type "HitResult Structure (by ref)"))
  ;[1 1 1] Smoke Damage
  (bind _asbasic_enemy_character (cast `BasicEnemyCharacter` OtherActor))
  (`BasicEnemyCharacter.SmokeStun` _asbasic_enemy_character (`self.smokeDurationMultiplier`)))

(event `self.Blocker.OnComponentBeginOverlap`
  (params (OverlappedComponent :type "PrimitiveComponent Object Reference") (OtherActor :type "Actor Object Reference") (OtherComp :type "PrimitiveComponent Object Reference") (OtherBodyIndex :type Integer) (bFromSweep :type Boolean) (SweepResult :type "HitResult Structure (by ref)"))
  (bind _ashero_animation_bp (cast `/Game/Characters/Sankari/Blueprints/HeroAnimationBP` (`SkeletalMeshComponent.GetAnimInstance` (`self.Mesh`)) :!pure true))
  ;[1 1 1] Blocking and countering
  (if (and (!= OtherActor self) (`HeroAnimator.blocking` _ashero_animation_bp) (not (`HeroAnimator.countering` _ashero_animation_bp)))
    (bind _asenemy_character (cast `EnemyCharacter` OtherActor))
    (bind _output_get (set `self.lastBlockedEnemy` _asenemy_character))
    (`self.AddBlockedDamager` OtherComp)
    (`self.BlockAttack` _output_get)
    (if (not (`self.counterEnabled`))
      (set `self.counterEnabled` true)
      (`KismetSystemLibrary.PrintString` "Counter!")
      (`KismetSystemLibrary.Delay` (`self.counterPromptTime`))
      (set `self.counterEnabled` false)
      (`KismetSystemLibrary.PrintString` "Too late"))))

(event `self.OnBlockStarted`
  ;[1 1 1] Blocking and countering
  (`PrimitiveComponent.SetCollisionEnabled` (`self.Blocker`) "QueryOnly"))

(event `self.OnBlockEnded`
  ;[1 1 1] Blocking and countering
  (`PrimitiveComponent.SetCollisionEnabled` (`self.Blocker`) "NoCollision"))

(fn `EnableAxe`
  (params (enable :type Boolean))
  (bind _damager (`self.Damager`))
  (if enable
    (`PrimitiveComponent.SetCollisionEnabled` _damager "QueryOnly")
    (else
      (`PrimitiveComponent.SetCollisionEnabled` _damager "NoCollision"))))

(fn `UserConstructionScript`)