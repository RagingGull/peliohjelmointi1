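; Base Behavior Tree task for the Pohatta character's AI.
; On execute, it caches the owning PohattaControllerBP and its controlled PohattaBP pawn if either reference is invalid.
; It then calls PerformTask and finishes with that result as success or failure.
; PerformTask is a stub that always returns true, apparently meant as an override point for child tasks.
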(event `self.ReceiveExecute`
  (params (OwnerActor :type "Actor Object Reference"))
  (bind _aspohatta_controller_bp (cast `/Game/Characters/Pohatta/Blueprints/PohattaControllerBP` OwnerActor :!pure true))
  (if (not (and (`KismetSystemLibrary.IsValid` (`self.Pohatta`)) (`KismetSystemLibrary.IsValid` (`self.Controller`))))
    (set `self.Controller` _aspohatta_controller_bp)
    (set `self.Pohatta` (cast `/Game/Characters/Pohatta/Blueprints/PohattaBP` (`Controller.K2_GetPawn` _aspohatta_controller_bp) :!pure true)))
  (bind _success (`self.PerformTask`))
  (`self.FinishExecute` _success))

(fn `PerformTask`
  (returns (success :type Boolean))
  (return true))