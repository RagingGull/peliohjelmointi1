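; PohattaBlock is an AI task for the Pohatta character that starts or releases blocking, depending on its Release flag.
; A release request fails early when Pohatta is not blocking; otherwise it calls Block with the inverse of Release.
; On a successful call it writes the current game time to the LastActionKey blackboard value and returns the result.
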(fn `PerformTask`
  (returns (success :type Boolean))
  (if (and (not (`BossCharacter.isBlocking` (`self.Pohatta`))) (`self.release`))
    (return false)
    (else
      (bind _success (`/Game/Characters/Pohatta/Blueprints/PohattaBP.Block` (`self.Pohatta`) (not (`self.release`))))
      (if _success
        (`BTFunctionLibrary.SetBlackboardValueAsFloat` (`self.lastActionKey`) (`GameplayStatics.GetTimeSeconds`)))
      (return _success))))