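; AI task for the Pohatta character that triggers its secondary attack once the primary attack count reaches three.
; PerformTask reads the count from the blackboard and calls AttackSecondary on Pohatta only when it equals exactly three.
; On success it records the current time as the last action and resets the count to zero.
; It returns whether the attack succeeded, or false when the count does not match.
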(fn `PerformTask`
  (returns (success :type Boolean))
  (if (== (`BTFunctionLibrary.GetBlackboardValueAsInt` (`self.PrimaryAttackCountKey`)) 3)
    (bind _success (`/Game/Characters/Pohatta/Blueprints/PohattaBP.AttackSecondary` (`self.Pohatta`)))
    (if _success
      (`BTFunctionLibrary.SetBlackboardValueAsFloat` (`self.LastActionKey`) (`GameplayStatics.GetTimeSeconds`))
      (`BTFunctionLibrary.SetBlackboardValueAsInt` (`self.PrimaryAttackCountKey`)))
    (return _success)
    (else
      (return false))))