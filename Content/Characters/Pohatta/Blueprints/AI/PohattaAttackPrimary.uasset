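; Pohatta AI task that makes the character perform its primary attack, limited by a counter on the Blackboard.
; PerformTask attacks only while the primary attack count is below three, otherwise it fails.
; A successful attack records the game time as the last action and increments the count, and the task returns the attack's result.
; The counter is not reset here.
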(fn `PerformTask`
  (returns (success :type Boolean))
  (bind _primaryattackcountkey (`self.primaryAttackCountKey`))
  (if (< (`BTFunctionLibrary.GetBlackboardValueAsInt` (`self.primaryAttackCountKey`)) 3)
    (bind _success (`/Game/Characters/Pohatta/Blueprints/PohattaBP.AttackPrimary` (`self.Pohatta`)))
    (if _success
      (`BTFunctionLibrary.SetBlackboardValueAsFloat` (`self.LastActionKey`) (`GameplayStatics.GetTimeSeconds`))
      (`BTFunctionLibrary.SetBlackboardValueAsInt` _primaryattackcountkey (+ (`BTFunctionLibrary.GetBlackboardValueAsInt` _primaryattackcountkey) 1)))
    (return _success)
    (else
      (return false))))