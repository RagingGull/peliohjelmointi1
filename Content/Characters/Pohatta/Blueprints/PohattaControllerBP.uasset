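; PohattaControllerBP is the AI controller for the Pohatta character, setting up its behavior when it possesses a pawn.
; On possess it casts the pawn to PohattaBP and, only if AI is enabled on it, initializes the PohattaBB blackboard.
; It copies the pawn's attack distances, reaction time, cooldown and Y boundary into blackboard keys, resets the attack count, then runs PohattaBT.
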(event `self.OnPossess`
  (params (PossessedPawn :type "Pawn Object Reference"))
  (bind _controllee (`self.Controllee`))
  (bind _controllee_2 (`self.Controllee`))
  (bind _output_get (set `self.Controllee` (cast `/Game/Characters/Pohatta/Blueprints/PohattaBP` PossessedPawn :!pure true)))
  (if (`EnemyCharacter.AIEnabled` _output_get)
    (bind _blackboardcomponent (`self.UseBlackboard` "/Game/Characters/Pohatta/Blueprints/AI/PohattaBB.PohattaBB"))
    (`BlackboardComponent.SetValueAsFloat` _blackboardcomponent (`self.PrimaryDistanceKey`) (`/Game/Characters/Pohatta/Blueprints/PohattaBP.attackDistancePrimary` _controllee_2))
    (`BlackboardComponent.SetValueAsFloat` _blackboardcomponent (`self.SecondaryDistanceKey`) (`/Game/Characters/Pohatta/Blueprints/PohattaBP.attackDistanceSecondary` _controllee_2))
    (`BlackboardComponent.SetValueAsFloat` _blackboardcomponent (`self.ReactionKey`) (`EnemyCharacter.reactionTime` _controllee))
    (`BlackboardComponent.SetValueAsFloat` _blackboardcomponent (`self.CooldownKey`) (`EnemyCharacter.attackCooldown` _controllee))
    (`BlackboardComponent.SetValueAsFloat` _blackboardcomponent (`self.BoundaryKey`) (`/Game/Characters/Pohatta/Blueprints/PohattaBP.boundaryY` _controllee))
    (`BlackboardComponent.SetValueAsInt` _blackboardcomponent (`self.attackCountKey`) 0)
    (`self.RunBehaviorTree` "/Game/Characters/Pohatta/Blueprints/AI/PohattaBT.PohattaBT")))

(fn `UserConstructionScript`)