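; Pohatta enemy character Blueprint that fights the hero with primary and secondary attacks and blocking, and whose death wins the game.
; Actions start only from Idle and trigger the anim Blueprint, whose attack-begin event resets a one-hit-per-attack guard for damager overlaps.
; Taking damage rescales a 3D health bar, and a successful block disrupts the hero's attack.
; Death ragdolls the mesh, drops physics-simulated equipment and replaces the HUD with a Victory screen.
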(event `self.ReceiveBeginPlay`
  ;[1 1 1] Init
  (`/Engine/EditorBlueprintResources/StandardMacros.IsValid` (`self.Anim`)
    (:`Is Valid`
      _)
    (:`Is Not Valid`
      (bind _output_get (set `self.Anim` (cast `/Game/Characters/Pohatta/Blueprints/PohattaAnimBP` (`SkeletalMeshComponent.GetAnimInstance` (`self.Mesh`)) :!pure true)))))
  (add `/Game/Characters/Pohatta/Blueprints/PohattaAnimBP.OnAnyAttackBegin` _output_get (delegate `OnAttack`)))

(event `OnAttack`
  ;[1 1 1] Init
  (set `self.hitHero` false)
  (bind _returnvalue (`self.FindHero`))
  (`HeroCharacter.RemoveBlockedDamager` _returnvalue (`self.Damager`)))

(event `self.Damager.OnComponentBeginOverlap`
  (params (OverlappedComponent :type "PrimitiveComponent Object Reference") (OtherActor :type "Actor Object Reference") (OtherComp :type "PrimitiveComponent Object Reference") (OtherBodyIndex :type Integer) (bFromSweep :type Boolean) (SweepResult :type "HitResult Structure (by ref)"))
  ;[1 1 1] Damage
  (bind _ashero_bp (cast `/Game/Characters/Sankari/Blueprints/HeroBP` OtherActor))
  (if (and (not (`self.hitHero`)) (not (`|EnumEquality` (`PrimitiveComponent.GetCollisionObjectType` OtherComp) "ECC_GameTraceChannel2")))
    (set `self.hitHero` true)
    (set `self.activeDamager` (`self.Damager`))
    (`GameplayStatics.ApplyDamage` _ashero_bp (select `bool` (`self.isAttackPrimary`) :`false` (`self.secondaryDamage`) :`true` (`self.primaryDamage`)) (`self.GetController`) self "/Script/Engine.DamageType")))

(event `self.Kill`
  (params (dmgType :type "DamageType Class Reference"))
  (bind _returnvalue (`GameplayStatics.GetPlayerController` 0))
  (bind _mesh (`self.Mesh`))
  ;[1 1 1] Death
  (`PrimitiveComponent.SetCollisionEnabled` _mesh "QueryAndPhysics")
  (`PrimitiveComponent.SetSimulatePhysics` _mesh true)
  (`self.SetDead` true)
  (set `self.state` "ES_Dead")
  (`SceneComponent.SetVisibility` (`self.HealthFill`) false false)
  (`SceneComponent.SetVisibility` (`self.HealthBg`) false false)
  (`self.DetachEquipment` (`self.Nuija`))
  (`self.DetachEquipment` (`self.sikari`))
  (`Widget.RemoveFromParent` (`/Game/Characters/Sankari/Blueprints/HeroBP.hud` (cast `/Game/Characters/Sankari/Blueprints/HeroBP` (`GameplayStatics.GetPlayerCharacter` 0) :!pure true)))
  (bind _returnvalue_2 (`|CreateWidget` "/Game/Menus/Victory.Victory_C"))
  (`UserWidget.AddToViewport` _returnvalue_2 0)
  (`WidgetBlueprintLibrary.SetInputMode_UIOnlyEx` _returnvalue _returnvalue_2)
  (set `PlayerController.bShowMouseCursor` true _returnvalue))

(event `self.ReceiveAnyDamage`
  (params (Damage :type "Float (single-precision)") (DamageType :type "DamageType Object Reference") (InstigatedBy :type "Controller Object Reference") (DamageCauser :type "Actor Object Reference"))
  ;[1 1 1] Healthbar
  (`KismetSystemLibrary.Delay` 0.1)
  (`SceneComponent.SetRelativeScale3D` (`self.HealthFill`) (`KismetMathLibrary.MakeVector` (`self.getHitpointRatio`) 1.0 1.0)))

(event `self.OnBlocked`
  (`/Game/Characters/Sankari/Blueprints/HeroBP.DisruptAttack` (cast `/Game/Characters/Sankari/Blueprints/HeroBP` (`GameplayStatics.GetPlayerPawn` 0) :!pure true)))

(fn `AttackPrimary`
  (returns (success :type Boolean))
  (bind _success (`self.CanStartAction`))
  (bind _output_get (set `/Game/Characters/Pohatta/Blueprints/PohattaAnimBP.attackPrimaryTrigger` _success (`self.Anim`)))
  (if _output_get
    (set `self.isAttackPrimary` true))
  (return _output_get))

(fn `AttackSecondary`
  (returns (success :type Boolean))
  (bind _success (`self.CanStartAction`))
  (bind _output_get (set `/Game/Characters/Pohatta/Blueprints/PohattaAnimBP.attackSecondaryTrigger` _success (`self.Anim`)))
  (if _output_get
    (set `self.isAttackPrimary` false))
  (return _output_get))

(fn `Block`
  (params (enable :type Boolean))
  (returns (success :type Boolean))
  (if enable
    (bind _success (`self.CanStartAction`))
    (if _success
      (set `self.isBlocking` true))
    (return _success)
    (else
      (set `self.isBlocking` false)
      (return true))))

(fn `CanStartAction`
  (returns (success :type Boolean))
  (return (`|EnumEquality` (`self.state`) "ES_Idle")))

(fn `DetachEquipment`
  (params (equipment :type "PrimitiveComponent Object Reference"))
  (`SceneComponent.K2_DetachFromComponent` equipment "KeepWorld" "KeepWorld" "KeepRelative" true)
  (`PrimitiveComponent.SetSimulatePhysics` equipment true)
  (`PrimitiveComponent.SetCollisionEnabled` equipment "QueryAndPhysics"))

(fn `EnableDamager`
  (params (enable :type Boolean))
  (`PrimitiveComponent.SetCollisionEnabled` (`self.Damager`) (select `bool` enable :`false` "NoCollision" :`true` "QueryOnly" :!type "ECollisionEnabled Enum")))

(fn `UserConstructionScript`)