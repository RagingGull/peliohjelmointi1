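; AI controller for the FeministiBP character that starts its behavior tree and steers it toward a target.
; On BeginPlay it sets up FeministBB, caches the controlled pawn, seeds the target key with the pawn's current location and runs FeministBT.
; UpdateTarget stores a new target and drives movement through the pawn's own GetDirection and Move functions.
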(event `self.ReceiveBeginPlay`
  (`self.UseBlackboard` "/Game/Characters/Feministi/Blueprints/FeministBB.FeministBB")
  (bind _output_get (set `self.feminist` (cast `/Game/Characters/Feministi/Blueprints/FeministiBP` (`self.K2_GetPawn`) :!pure true)))
  (`BlackboardComponent.SetValueAsVector` (`AIBlueprintHelperLibrary.GetBlackboard` self) (`self.targetKey`) (`self.K2_GetActorLocation` _output_get))
  (`self.RunBehaviorTree` "/Game/Characters/Feministi/Blueprints/FeministBT.FeministBT"))

(fn `UpdateTarget`
  (params (target :type "Vector Structure"))
  (bind _output_get (set `self.Target` target))
  (`TwoDirectionalCharacter.Move` (`self.feminist`) (`TwoDirectionalCharacter.GetDirection` (`self.feminist`) _output_get)))

(fn `UserConstructionScript`)