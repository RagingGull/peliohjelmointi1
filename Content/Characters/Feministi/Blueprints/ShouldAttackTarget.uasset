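; Behavior tree decorator for the Feministi AI that checks whether its target is within attack range.
; It caches the owning FeministController, then compares the controlled pawn's distance from the target location vector in the blackboard against a blackboard attack distance.
; The condition passes only when that distance is strictly less than the attack distance.
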(fn `PerformConditionCheck`
  (params (OwnerActor :type "Actor Object Reference"))
  (returns (ReturnValue :type Boolean))
  (`/Engine/EditorBlueprintResources/StandardMacros.IsValid` (`self.AICon`)
    (:`Is Valid`
      _)
    (:`Is Not Valid`
      (bind _output_get (set `self.AICon` (cast `/Game/Characters/Feministi/Blueprints/FeministController` OwnerActor :!pure true)))))
  (return (< (`KismetMathLibrary.VSize` (- (`Actor.K2_GetActorLocation` (`Controller.K2_GetPawn` _output_get)) (`BTFunctionLibrary.GetBlackboardValueAsVector` (`self.targetKey`)))) (`BTFunctionLibrary.GetBlackboardValueAsFloat` (`self.attackDistanceKey`)))))