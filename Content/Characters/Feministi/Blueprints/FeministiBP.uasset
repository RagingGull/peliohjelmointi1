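; FeministiBP is the Blueprint for the Feministi character, relaying action flags to its animation Blueprint, FeministAnimBP.
; Each Tick, Atk and Dodge act as one-shot flags that reset and trigger Attack or Dodge on the mesh's anim instance.
; Duck acts as a held state, calling Duck while true and StopDucking otherwise, every frame.
; An unconnected node for simulating hair bone physics never runs.
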(event `self.ReceiveBeginPlay`)

(event `self.ReceiveTick`
  (params (DeltaSeconds :type "Float (single-precision)"))
  (bind _asfeminist_anim_bp (cast `/Game/Characters/Feministi/Blueprints/FeministAnimBP` (`SkeletalMeshComponent.GetAnimInstance` (`self.Mesh`)) :!pure true))
  (`|ExecutionSequence`
    (:`then_0`
      (if (`self.atk`)
        (set `self.atk` false)
        (`/Game/Characters/Feministi/Blueprints/FeministAnimBP.Attack` _asfeminist_anim_bp)))
    (:`then_1`
      (if (`self.dodge`)
        (set `self.dodge` false)
        (`/Game/Characters/Feministi/Blueprints/FeministAnimBP.Dodge` _asfeminist_anim_bp)))
    (:`then_2`
      (if (`self.duck`)
        (`/Game/Characters/Feministi/Blueprints/FeministAnimBP.Duck` _asfeminist_anim_bp)
        (else
          (`/Game/Characters/Feministi/Blueprints/FeministAnimBP.StopDucking` _asfeminist_anim_bp))))))

(fn `UserConstructionScript`)