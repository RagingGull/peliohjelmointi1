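; DeadVertBP is a character death actor with two halves that physically fall apart, judging by its name a vertical split.
; On the second completion notification it enables physics on both halves, destroys the notifying source actor and starts a looping timer at frame-delta interval.
; The timer pushes the halves in opposite directions along world X from a point above the actor's origin, stopping after just under a second.
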(fn `NotifyOfCompletion`
  (params (Source :type "Actor Object Reference"))
  (bind _result (`/Engine/EditorBlueprintResources/StandardMacros.IncrementInt` (`self.completedCounter`))
    (:`  `
      (if (== _result 2)
        (`PrimitiveComponent.SetSimulatePhysics` (`self.FirstHalf`) true)
        (`PrimitiveComponent.SetSimulatePhysics` (`self.SecondHalf`) true)
        (`self.K2_DestroyActor` Source)
        (bind _returnvalue (`KismetSystemLibrary.K2_SetTimer` null "Push" (`GameplayStatics.GetWorldDeltaSeconds`) true))
        (set `self.PushTimer` _returnvalue)))))

(fn `Push`
  (bind _returnvalue (* (`KismetMathLibrary.MakeVector` 1.0) (`self.PushForce`)))
  (bind _returnvalue_2 (+ (`self.K2_GetActorLocation`) (0.0 0.0 100.0)))
  (if (== (`self.PushStartTime`) 0.0)
    (set `self.PushStartTime` (`GameplayStatics.GetTimeSeconds`)))
  (`PrimitiveComponent.AddForceAtLocation` (`self.FirstHalf`) _returnvalue _returnvalue_2 "None")
  (`PrimitiveComponent.AddForceAtLocation` (`self.SecondHalf`) (* _returnvalue -1.0) _returnvalue_2 "None")
  (if (> (- (`GameplayStatics.GetTimeSeconds`) (`self.PushStartTime`)) 0.9)
    (`KismetSystemLibrary.K2_ClearAndInvalidateTimerHandle` (`self.PushTimer`))))

(fn `UserConstructionScript`
  (`parent.UserConstructionScript`))