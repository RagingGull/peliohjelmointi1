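; DeadHorizontalBP is a character death actor with two body halves, apparently for a horizontal cut.
; It counts completion notifications through NotifyOfCompletion, whose senders are not shown in this graph.
; When the counter check reaches two, it enables physics simulation on both halves and destroys the Source actor passed in that call.
; The construction script only runs the parent's.
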(fn `NotifyOfCompletion`
  (params (Source :type "Actor Object Reference"))
  (bind _result (`/Engine/EditorBlueprintResources/StandardMacros.IncrementInt` (`self.completedCounter`))
    (:`  `
      (if (== _result 2)
        (`PrimitiveComponent.SetSimulatePhysics` (`self.FirstHalf`) true)
        (`PrimitiveComponent.SetSimulatePhysics` (`self.SecondHalf`) true)
        (`self.K2_DestroyActor` Source)))))

(fn `UserConstructionScript`
  (`parent.UserConstructionScript`))