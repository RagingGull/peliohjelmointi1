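; Enemy spawner actor that releases a set number of enemies at a spawn point once the hero enters its trigger.
; The HeroBP overlap disables the trigger collider, spawns one EnemyClass immediately and starts a looping timer that spawns another each interval.
; A counter stops spawning and clears the timer when it reaches Num.
; ResetAll zeroes the counter and re-arms the trigger for reuse.
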(event `self.SpawnTrigger.OnComponentBeginOverlap`
  (params (OverlappedComponent :type "PrimitiveComponent Object Reference") (OtherActor :type "Actor Object Reference") (OtherComp :type "PrimitiveComponent Object Reference") (OtherBodyIndex :type Integer) (bFromSweep :type Boolean) (SweepResult :type "HitResult Structure (by ref)"))
  (if (and (== (`GameplayStatics.GetObjectClass` OtherActor) "/Game/Characters/Sankari/Blueprints/HeroBP.HeroBP_C") (`self.SpawningEnabled`))
    (`self.EnableSpawnCollider` false)
    (`self.SpawnOne`)
    (bind _returnvalue (`KismetSystemLibrary.K2_SetTimerDelegate` (delegate `SpawnOne`) (`self.Interval`) true))))

(event `SpawnOne`
  (if (`self.SpawningEnabled`)
    (`|SpawnActorFromClass` (`self.EnemyClass`) (`SceneComponent.K2_GetComponentToWorld` (`self.SpawnPoint`)) "AdjustIfPossibleButAlwaysSpawn" "OverrideRootScale")
    (bind _result (`/Engine/EditorBlueprintResources/StandardMacros.IncrementInt` (`self.enemiesSpawned`))
      (:`  `
        (if (== _result (`self.Num`))
          (set `self.SpawningEnabled` false)
          (`KismetSystemLibrary.K2_ClearAndInvalidateTimerHandle` (stale `self.SpawnTrigger.OnComponentBeginOverlap` _returnvalue)))))))

(fn `EnableSpawnCollider`
  (params (enable :type Boolean))
  (`PrimitiveComponent.SetCollisionEnabled` (`self.SpawnTrigger`) (select `bool` enable :`false` (enumliteral `ECollisionEnabled` "NoCollision") :`true` "QueryOnly")))

(fn `ResetAll`
  (set `self.enemiesSpawned` 0)
  (set `self.SpawningEnabled` true)
  (`self.EnableSpawnCollider` true))

(fn `UserConstructionScript`)