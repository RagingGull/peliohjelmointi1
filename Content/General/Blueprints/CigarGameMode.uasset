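; CigarGameMode is a game mode that handles checkpoint-based player spawning.
; SetCheckpoint stores the last checkpoint, which ChoosePlayerStart returns as the spawn point while it is valid.
; With no valid checkpoint, it searches the PlayerStart actors for the "Initial" tag and caches that one as the checkpoint.
; Restarting a player resets global time dilation to normal speed.
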(event `self.K2_OnRestartPlayer`
  (params (NewPlayer :type "Controller Object Reference"))
  (`GameplayStatics.SetGlobalTimeDilation` 1.0))

(fn `ChoosePlayerStart`
  (params (Player :type "Controller Object Reference"))
  (returns (ReturnValue :type "Actor Object Reference"))
  (bind _lastcheckpoint (`self.lastCheckPoint`))
  (`/Engine/EditorBlueprintResources/StandardMacros.IsValid` _lastcheckpoint
    (:`Is Valid`
      (return _lastcheckpoint))
    (:`Is Not Valid`
      (bind _outactors (`GameplayStatics.GetAllActorsOfClass` "/Script/Engine.PlayerStart"))
      (for _array_element _outactors
        (if (== (`PlayerStart.PlayerStartTag` _array_element) "Initial")
          (set `self.lastCheckPoint` _array_element)
          (break)))
      (return (`self.lastCheckPoint`)))))

(fn `SetCheckpoint`
  (params (cp :type "Actor Object Reference"))
  (set `self.lastCheckPoint` cp))

(fn `UserConstructionScript`)