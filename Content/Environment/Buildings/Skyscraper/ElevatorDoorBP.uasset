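; Skyscraper elevator door Blueprint that slides two door panels apart when something overlaps its trigger and back together when the overlap ends.
; Each overlap event sets the direction flag and starts a looping timer, using frame delta as its interval, that calls DoorLoop.
; DoorLoop moves LeftDoor and RightDoor in opposite Y directions at constant speed, clearing the timer once LeftDoor passes its open or closed limit.
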(event `self.Trigger.OnComponentBeginOverlap`
  (params (OverlappedComponent :type "PrimitiveComponent Object Reference") (OtherActor :type "Actor Object Reference") (OtherComp :type "PrimitiveComponent Object Reference") (OtherBodyIndex :type Integer) (bFromSweep :type Boolean) (SweepResult :type "HitResult Structure (by ref)"))
  (set `self.DoorDirection` true)
  (bind _returnvalue (`KismetSystemLibrary.K2_SetTimer` null "DoorLoop" (`GameplayStatics.GetWorldDeltaSeconds`) true :!label _label))
  (set `self.DoorTimer` _returnvalue))

(event `self.Trigger.OnComponentEndOverlap`
  (params (OverlappedComponent :type "PrimitiveComponent Object Reference") (OtherActor :type "Actor Object Reference") (OtherComp :type "PrimitiveComponent Object Reference") (OtherBodyIndex :type Integer))
  (set `self.DoorDirection` false)
  (goto _label))

(fn `DoorLoop`
  (bind _returnvalue (* (`GameplayStatics.GetWorldDeltaSeconds`) 40.0))
  (bind (_relativelocation_x _relativelocation_y) (`KismetMathLibrary.BreakVector` (`SceneComponent.RelativeLocation` (`self.LeftDoor`))))
  (bind _returnvalue_2 (select `bool` (`self.DoorDirection`) :`false` (* _returnvalue -1.0) :`true` _returnvalue))
  (`SceneComponent.K2_AddRelativeLocation` (`self.LeftDoor`) (`KismetMathLibrary.MakeVector` 0.0 (* _returnvalue_2 -1.0)) false false)
  (`SceneComponent.K2_AddRelativeLocation` (`self.RightDoor`) (`KismetMathLibrary.MakeVector` 0.0 _returnvalue_2) false false)
  (if (`self.DoorDirection`)
    (if (<= _relativelocation_y -110.0)
      (`KismetSystemLibrary.K2_ClearAndInvalidateTimerHandle` (`self.DoorTimer`) :!label _label))
    (elif (>= _relativelocation_y -40.0)
      (goto _label))))

(fn `UserConstructionScript`)