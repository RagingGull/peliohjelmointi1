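; Cigar store building Blueprint with player-operated double doors and a trigger that ends level 1.
; DoorTrigger shows an open/close HUD hint and enables Interact input; ToggleDoor picks a direction from the left door's yaw, and a looping frame-delta timer swings both doors oppositely.
; The Inside volume changes the hero's camera distance on entry and exit.
; EventTrigger pauses the game and replaces the HUD with the Level1Finish screen.
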(event `self.DoorTrigger.OnComponentEndOverlap`
  (params (OverlappedComponent :type "PrimitiveComponent Object Reference") (OtherActor :type "Actor Object Reference") (OtherComp :type "PrimitiveComponent Object Reference") (OtherBodyIndex :type Integer))
  (set `self.toggleEnabled` false)
  (`/Game/HUD/IngameHUD.HideInfo` (`self.HudRef`))
  (`self.DisableInput` (`GameplayStatics.GetPlayerController` 0)))

(event `self.DoorTrigger.OnComponentBeginOverlap`
  (params (OverlappedComponent :type "PrimitiveComponent Object Reference") (OtherActor :type "Actor Object Reference") (OtherComp :type "PrimitiveComponent Object Reference") (OtherBodyIndex :type Integer) (bFromSweep :type Boolean) (SweepResult :type "HitResult Structure (by ref)"))
  (bind _ashero_bp (cast `/Game/Characters/Sankari/Blueprints/HeroBP` OtherActor))
  (set `self.toggleEnabled` true)
  (bind _output_get (set `self.HudRef` (`/Game/Characters/Sankari/Blueprints/HeroBP.hud` _ashero_bp)))
  (`/Game/HUD/IngameHUD.DisplayInfo` _output_get 0.0 (select `bool` (`self.doorDirection`) :`false` (`self.InfoToOpen`) :`true` (`self.InfoToClose`)))
  (`self.EnableInput` (`GameplayStatics.GetPlayerController` 0)))

(event `InputAction|Interact`
  (params (Key :type "Key Structure" :default "AnyKey"))
  (:`Pressed`
    (if (`self.toggleEnabled`)
      (`self.ToggleDoor`)
      (set `/Game/HUD/IngameHUD.infoText` (select `bool` (`self.doorDirection`) :`false` (`self.InfoToOpen`) :`true` (`self.InfoToClose`)) (`self.HudRef`)))))

(event `self.EventTrigger.OnComponentBeginOverlap`
  (params (OverlappedComponent :type "PrimitiveComponent Object Reference") (OtherActor :type "Actor Object Reference") (OtherComp :type "PrimitiveComponent Object Reference") (OtherBodyIndex :type Integer) (bFromSweep :type Boolean) (SweepResult :type "HitResult Structure (by ref)"))
  (bind _returnvalue (`GameplayStatics.GetPlayerController` 0))
  (`GameplayStatics.SetGamePaused` true)
  (`Widget.RemoveFromParent` (`self.HudRef`))
  (bind _returnvalue_2 (`|CreateWidget` "/Game/Menus/Level1Finish.Level1Finish_C"))
  (`UserWidget.AddToViewport` _returnvalue_2 0)
  (`WidgetBlueprintLibrary.SetInputMode_UIOnlyEx` _returnvalue _returnvalue_2)
  (set `PlayerController.bShowMouseCursor` true _returnvalue))

(event `self.Inside.OnComponentBeginOverlap`
  (params (OverlappedComponent :type "PrimitiveComponent Object Reference") (OtherActor :type "Actor Object Reference") (OtherComp :type "PrimitiveComponent Object Reference") (OtherBodyIndex :type Integer) (bFromSweep :type Boolean) (SweepResult :type "HitResult Structure (by ref)"))
  (bind _ashero_bp (cast `/Game/Characters/Sankari/Blueprints/HeroBP` OtherActor))
  (`/Game/Characters/Sankari/Blueprints/HeroBP.ChangeCamDistance` _ashero_bp 300.0))

(event `self.Inside.OnComponentEndOverlap`
  (params (OverlappedComponent :type "PrimitiveComponent Object Reference") (OtherActor :type "Actor Object Reference") (OtherComp :type "PrimitiveComponent Object Reference") (OtherBodyIndex :type Integer))
  (bind _ashero_bp (cast `/Game/Characters/Sankari/Blueprints/HeroBP` OtherActor))
  (`/Game/Characters/Sankari/Blueprints/HeroBP.ChangeCamDistance` _ashero_bp 500.0))

(fn `DoorLoop`
  (bind _doorleft (`self.DoorLeft`))
  (bind _doorright (`self.DoorRight`))
  (bind _returnvalue (* (`GameplayStatics.GetWorldDeltaSeconds`) 60.0))
  (bind (_relativerotation_roll _relativerotation_pitch _relativerotation_yaw) (`KismetMathLibrary.BreakRotator` (`SceneComponent.RelativeRotation` (`self.DoorLeft`))))
  (bind _returnvalue_2 (`KismetMathLibrary.MakeRotator` 0.0 0.0 _returnvalue))
  (bind _returnvalue_3 (`KismetMathLibrary.MakeRotator` 0.0 0.0 (* _returnvalue -1.0)))
  (if (`self.doorDirection`)
    (`SceneComponent.K2_AddRelativeRotation` _doorleft _returnvalue_2 false false)
    (`SceneComponent.K2_AddRelativeRotation` _doorright _returnvalue_3 false false)
    (if (>= _relativerotation_yaw 100.0)
      (`KismetSystemLibrary.K2_ClearAndInvalidateTimerHandle` (`self.DoorTimer`) :!label _label))
    (else
      (`SceneComponent.K2_AddRelativeRotation` _doorleft _returnvalue_3 false false)
      (`SceneComponent.K2_AddRelativeRotation` _doorright _returnvalue_2 false false)
      (if (<= _relativerotation_yaw 0.5)
        (goto _label)))))

(fn `ToggleDoor`
  (bind (_relativerotation_roll _relativerotation_pitch _relativerotation_yaw) (`KismetMathLibrary.BreakRotator` (`SceneComponent.RelativeRotation` (`self.DoorLeft`))))
  (set `self.doorDirection` (< _relativerotation_yaw 3.0))
  (bind _returnvalue (`KismetSystemLibrary.K2_SetTimer` null "DoorLoop" (`GameplayStatics.GetWorldDeltaSeconds`) true))
  (set `self.DoorTimer` _returnvalue))

(fn `UserConstructionScript`)